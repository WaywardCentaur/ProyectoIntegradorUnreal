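; Blueprint function library that stores per-user blockchain wallets locally as B_Wallet_Savegame slots named after the user.
; Functions check, read and clear a wallet, or add unique entries to its token and local token path arrays.
; Each add loads any existing save, then writes a fresh save object carrying only the edited array.
; As a result, adding a token drops saved paths, and adding a path drops saved tokens.
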(fn WalletExists
  (params (WalletName :type String))
  (bind _returnvalue (SaveGame|DoesSaveGameExist WalletName))
  (return _returnvalue))

(fn WalletAdd
  (params (User%20name :type String) (New%20token :type String))
  (bind _returnvalue (SaveGame|DoesSaveGameExist User%20name))
  (if _returnvalue
    (bind _returnvalue_2 (SaveGame|LoadGamefromSlot User%20name))
    (bind _asb_wallet_savegame (Utilities|Casting|CastToB_Wallet_Savegame _returnvalue_2))
    (Utilities|Array|AddUnique (Variables|/Game/Blockchain/Blueprints/B_Wallet_Savegame.B_Wallet_Savegame_C|GetTokens _asb_wallet_savegame) New%20token)
    (bind _returnvalue_3 (SaveGame|CreateSaveGameObject "/Game/Blockchain/Blueprints/B_Wallet_Savegame.B_Wallet_Savegame_C"))
    (Variables|/Game/Blockchain/Blueprints/B_Wallet_Savegame.B_Wallet_Savegame_C|SetTokens _returnvalue_3 (Variables|/Game/Blockchain/Blueprints/B_Wallet_Savegame.B_Wallet_Savegame_C|GetTokens _asb_wallet_savegame))
    (bind _returnvalue_4 (SaveGame|SaveGametoSlot _returnvalue_3 User%20name))
    (return _returnvalue_4)
    (else
      (bind _returnvalue_5 (SaveGame|CreateSaveGameObject "/Game/Blockchain/Blueprints/B_Wallet_Savegame.B_Wallet_Savegame_C"))
      (Variables|/Game/Blockchain/Blueprints/B_Wallet_Savegame.B_Wallet_Savegame_C|SetTokens _returnvalue_5 (Utilities|Array|MakeArray New%20token))
      (bind _returnvalue_6 (SaveGame|SaveGametoSlot _returnvalue_5 User%20name))
      (return _returnvalue_6))))

(fn WalletRead
  (params (user%20Name :type String))
  (bind _returnvalue (SaveGame|LoadGamefromSlot user%20Name))
  (bind _asb_wallet_savegame (Utilities|Casting|CastToB_Wallet_Savegame _returnvalue)
    (:then
      (return (Variables|/Game/Blockchain/Blueprints/B_Wallet_Savegame.B_Wallet_Savegame_C|GetTokens _asb_wallet_savegame) true))
    (:CastFailed
      (return 0 false))))

(fn ClearWallet
  (params (user%20Name :type String))
  (bind _returnvalue (SaveGame|DeleteGameinSlot user%20Name))
  (return _returnvalue))

(fn WalletAddPath
  (params (User%20name :type String) (New%20token%20path :type String))
  (bind _returnvalue (SaveGame|DoesSaveGameExist User%20name))
  (if _returnvalue
    (bind _returnvalue_2 (SaveGame|LoadGamefromSlot User%20name))
    (bind _asb_wallet_savegame (Utilities|Casting|CastToB_Wallet_Savegame _returnvalue_2))
    (Utilities|Array|AddUnique (Variables|/Game/Blockchain/Blueprints/B_Wallet_Savegame.B_Wallet_Savegame_C|GetTokenLocalPath _asb_wallet_savegame) New%20token%20path)
    (bind _returnvalue_3 (SaveGame|CreateSaveGameObject "/Game/Blockchain/Blueprints/B_Wallet_Savegame.B_Wallet_Savegame_C"))
    (Variables|/Game/Blockchain/Blueprints/B_Wallet_Savegame.B_Wallet_Savegame_C|SetTokenLocalPath _returnvalue_3 (Variables|/Game/Blockchain/Blueprints/B_Wallet_Savegame.B_Wallet_Savegame_C|GetTokenLocalPath _asb_wallet_savegame))
    (bind _returnvalue_4 (SaveGame|SaveGametoSlot _returnvalue_3 User%20name))
    (return _returnvalue_4)
    (else
      (bind _returnvalue_5 (SaveGame|CreateSaveGameObject "/Game/Blockchain/Blueprints/B_Wallet_Savegame.B_Wallet_Savegame_C"))
      (Variables|/Game/Blockchain/Blueprints/B_Wallet_Savegame.B_Wallet_Savegame_C|SetTokenLocalPath _returnvalue_5 (Utilities|Array|MakeArray New%20token%20path))
      (bind _returnvalue_6 (SaveGame|SaveGametoSlot _returnvalue_5 User%20name))
      (return _returnvalue_6))))

(fn WalletReadPath
  (params (user%20Name :type String))
  (bind _returnvalue (SaveGame|LoadGamefromSlot user%20Name))
  (bind _asb_wallet_savegame (Utilities|Casting|CastToB_Wallet_Savegame _returnvalue)
    (:then
      (return (Variables|/Game/Blockchain/Blueprints/B_Wallet_Savegame.B_Wallet_Savegame_C|GetTokenLocalPath _asb_wallet_savegame) true))
    (:CastFailed
      (return 0 false))))